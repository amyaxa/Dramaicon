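; BP_Elevator is a moving elevator actor that shuttles between StartPoint and EndPoint actors, starting on BeginPlay.
; ChooChoo uses a FlipFlop to alternately play and reverse the Rails timeline, which lerps actor location and re-triggers ChooChoo after a pause when finished.
; A separate Levitation timeline, started on BeginPlay, adds a vertical world offset on each update, with no sweep.
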(event `self.ReceiveBeginPlay`
  (`self.ChooChoo`)
  (bind (_direction _motion) (`Timeline|Levitation`)
    (:`Update`
      (`self.K2_AddActorWorldOffset` (`KismetMathLibrary.MakeVector` 0.0 0.0 _motion)))))

(event `ChooChoo`
  (`/Engine/EditorBlueprintResources/StandardMacros.FlipFlop`
    (:`A`
      (bind (_direction _motionpath) (`Timeline|Rails` :!via `PlayFromStart` :!label _label)
        (:`Update`
          (`self.K2_SetActorLocation` (`KismetMathLibrary.VLerp` (`self.K2_GetActorLocation` (`self.Start Point`)) (`self.K2_GetActorLocation` (`self.End Point`)) _motionpath)))
        (:`Finished`
          (`KismetSystemLibrary.Delay` 4.0)
          (`self.ChooChoo`))))
    (:`B`
      (goto _label :!via `ReverseFromEnd`))))

(fn `UserConstructionScript`)